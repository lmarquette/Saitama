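; BP_Spawn is a spawner that populates the level with up to 252 BP_AI pawns around its own position.
; Tick runs through a randomized short Delay, which throttles spawning to a staggered stream rather than one per frame.
; Each spawn gets a small random positive X offset from the actor's location and increments the SpawnAi counter until the cap stops it.
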(event EventTick
  (params (DeltaSeconds :type Float%20%28single-precision%29))
  (bind _returnvalue (Transformation|GetActorLocation))
  (bind (_x _y _z) (Math|Vector|BreakVector _returnvalue))
  (Utilities|FlowControl|Delay (Math|Random|RandomFloatinRange 0.1 0.2))
  (if (not (>= (Variables|Default|GetSpawn%20Ai) 252.0))
    (AI|SpawnAIFromClass "/Game/BP_AI.BP_AI_C" 0 (Math|Vector|MakeVector (+ _x (Math|Random|RandomFloatinRange 0.0 3e+01)) _y _z) "0, 0, 0" false)
    (Variables|Default|SetSpawn%20Ai (+ (Variables|Default|GetSpawn%20Ai) 1.0))))

(event Collision|EventActorBeginOverlap
  (params (OtherActor :type Actor%20Object%20Reference)))

(fn ConstructionScript)